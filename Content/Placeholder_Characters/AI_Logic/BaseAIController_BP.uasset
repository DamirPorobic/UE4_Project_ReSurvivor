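; Base AI controller for placeholder characters that runs the base behavior tree on BeginPlay.
; It caches the game instance and polls its paused flag every tick.
; While the game is paused it stops the brain component's logic, and restarts it once play resumes, using an AIEnabled flag to avoid repeated restarts.
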(event `self.ReceiveBeginPlay`
  (`self.RunBehaviorTree` "/Game/Placeholder_Characters/AI_Logic/BaseBehaviorTree.BaseBehaviorTree")
  (bind _asgame_instance_bp (cast `/Game/Blueprints/GameInstance_BP` (`GameplayStatics.GetGameInstance`)))
  (set `self.ReferenceToGameInstance` _asgame_instance_bp)
  (set `self.AIEnabled` true))

(event `self.ReceiveTick`
  (params (DeltaSeconds :type "Float (single-precision)"))
  (if (`/Game/Blueprints/GameInstance_BP.IsGamePaused` (`self.ReferenceToGameInstance`))
    (`BrainComponent.StopLogic` (`self.BrainComponent`) "")
    (set `self.AIEnabled` false)
    (elif (not (`self.AIEnabled`))
      (`BrainComponent.RestartLogic` (`self.BrainComponent`))
      (set `self.AIEnabled` true))))

(fn `UserConstructionScript`)