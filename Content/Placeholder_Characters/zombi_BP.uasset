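; Placeholder zombie AI pawn that wanders at random and moves toward the player when it sees them.
; Tick starts a move to a random reachable point whenever IsMoving is false, and that move's success or failure clears the flag.
; PawnSensing sets IsMoving for any seen pawn, then runs AIMoveTo on it if it is a FirstPersonCharacter_BP.
; The chase move never clears IsMoving itself.
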(event `self.PawnSensing.OnSeePawn`
  (params (Pawn :type "Pawn Object Reference"))
  (set `self.IsMoving` true)
  (bind _asfirst_person_character_bp (cast `/Game/Blueprints/FirstPersonCharacter_BP` Pawn))
  (`|AIMoveTo` self (0.0 0.0 0.0) _asfirst_person_character_bp))

(event `self.ReceiveTick`
  (params (DeltaSeconds :type "Float (single-precision)"))
  (if (not (`self.IsMoving`))
    (`|AIMoveTo` self (`NavigationSystem.GetRandomReachablePointInRadius` (`self.K2_GetActorLocation`))
      (:`then`
        (set `self.IsMoving` true))
      (:`OnSuccess`
        (set `self.IsMoving` false :!label _label))
      (:`OnFail`
        (goto _label)))))

(fn `UserConstructionScript`)