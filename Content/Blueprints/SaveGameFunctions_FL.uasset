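; Blueprint function library that saves and restores the first-person player's transform, inventory, files, equipped weapon with ammo, and health.
; Saving captures those stats plus map name and time, then writes a new slot or overwrites the current one, based on the game instance's new-game flag.
; A separate "Metadata" save indexes all slots with map and date.
; Loading reads the current slot and reapplies the stats, refreshing the HUD.
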(fn StorePlayerStats
  (params (SaveGameInput :type Save%20Game%20BP%20Object%20Reference) (OwningPlayer :type First%20Person%20Character%20BP%20Object%20Reference))
  (LocalVariables|SetSaveGameInstance SaveGameInput)
  (LocalVariables|SetOwningPlayerPawn OwningPlayer)
  (Utilities|FlowControl|Sequence
    (:then_0
      ;[1 1 1] Store data related only to the player pawn, like inventory, weapon, files and so on
      (Variables|/Game/Blueprints/SaveGame_BP.SaveGame_BP_C|SetPlayerRotation (LocalVariables|GetSaveGameInstance) (Pawn|GetControlRotation (LocalVariables|GetOwningPlayerPawn) :!class /Script/Engine.Pawn))
      (Variables|/Game/Blueprints/SaveGame_BP.SaveGame_BP_C|SetPlayerLocation (LocalVariables|GetSaveGameInstance) (Transformation|GetActorLocation (LocalVariables|GetOwningPlayerPawn)))
      (Variables|/Game/Blueprints/SaveGame_BP.SaveGame_BP_C|SetPlayerInventory (LocalVariables|GetSaveGameInstance) (Variables|/Game/Blueprints/FirstPersonCharacter_BP.FirstPersonCharacter_BP_C|GetInventory (LocalVariables|GetOwningPlayerPawn)))
      (Variables|/Game/Blueprints/SaveGame_BP.SaveGame_BP_C|SetPlayerFiles (LocalVariables|GetSaveGameInstance) (Variables|/Game/Blueprints/FirstPersonCharacter_BP.FirstPersonCharacter_BP_C|GetFileStorage (LocalVariables|GetOwningPlayerPawn)))
      (Variables|/Game/Blueprints/SaveGame_BP.SaveGame_BP_C|SetEquipedWeapon (LocalVariables|GetSaveGameInstance) (Variables|/Game/Blueprints/FirstPersonCharacter_BP.FirstPersonCharacter_BP_C|GetEquippedWeapon (LocalVariables|GetOwningPlayerPawn)))
      (Variables|/Game/Blueprints/SaveGame_BP.SaveGame_BP_C|SetLoadedAmmunition (LocalVariables|GetSaveGameInstance) (Variables|/Game/Placeholder_Assets/Actors/ItemBaseClass_Actor.ItemBaseClass_Actor_C|GetStackSize (Variables|/Game/Blueprints/FirstPersonCharacter_BP.FirstPersonCharacter_BP_C|GetEquippedWeapon (LocalVariables|GetOwningPlayerPawn))))
      (Variables|/Game/Blueprints/SaveGame_BP.SaveGame_BP_C|SetCurrentHealth (LocalVariables|GetSaveGameInstance) (Variables|/Game/Blueprints/FirstPersonCharacter_BP.FirstPersonCharacter_BP_C|GetCurrentHealth (LocalVariables|GetOwningPlayerPawn))))
    (:then_1
      ;[1 1 1] Store level and time related data
      (bind _returnvalue (Game|GetCurrentLevelName 0))
      (Variables|/Game/Blueprints/SaveGame_BP.SaveGame_BP_C|SetMapName (LocalVariables|GetSaveGameInstance) (Utilities|String|StringToName _returnvalue))
      (Variables|/Game/Blueprints/SaveGame_BP.SaveGame_BP_C|SetDateTime (LocalVariables|GetSaveGameInstance) (Math|DateTime|Now)))
    (:then_2
      (return (LocalVariables|GetSaveGameInstance)))))

(fn WritetoMemory
  (params (SaveGame :type Save%20Game%20BP%20Object%20Reference))
  (LocalVariables|SetSaveGameInstance SaveGame)
  ;[1 1 1] Get the game instance variable and see if this is a new game and if we are saving for the first time.
  (bind _asgame_instance_bp (Utilities|Casting|CastToGameInstance_BP (Game|GetGameInstance)))
  (bind _output_get (LocalVariables|SetGameInstance _asgame_instance_bp))
  (if (Variables|/Game/Blueprints/GameInstance_BP.GameInstance_BP_C|GetIsNewGame _output_get)
    (bind _slotname (CallFunction|AddNewtoMetadata (LocalVariables|GetSaveGameInstance)))
    (SaveGame|SaveGametoSlot (LocalVariables|GetSaveGameInstance) _slotname)
    (Variables|/Game/Blueprints/GameInstance_BP.GameInstance_BP_C|SetSaveGameSlotName (LocalVariables|GetGameInstance) _slotname)
    (Variables|/Game/Blueprints/GameInstance_BP.GameInstance_BP_C|SetIsNewGame (LocalVariables|GetGameInstance) false)
    (else
      (CallFunction|UpdateMetadataEntry (LocalVariables|GetSaveGameInstance) (Variables|/Game/Blueprints/GameInstance_BP.GameInstance_BP_C|GetSaveGameSlotName (LocalVariables|GetGameInstance)))
      (SaveGame|SaveGametoSlot (LocalVariables|GetSaveGameInstance) (Variables|/Game/Blueprints/GameInstance_BP.GameInstance_BP_C|GetSaveGameSlotName (LocalVariables|GetGameInstance))))))

(fn AddNewtoMetadata
  (params (SaveGame :type Save%20Game%20BP%20Object%20Reference))
  (LocalVariables|SetSaveGameInstance SaveGame)
  ;[1 1 1] Try to load the metadata file, if it's not possible (first time saving in game) then create a new file
  (bind _returnvalue (SaveGame|LoadGamefromSlot "Metadata"))
  (Utilities|IsValid _returnvalue
    (:Is%20Valid
      (bind _assave_game_metadata_bp (Utilities|Casting|CastToSaveGameMetadata_BP _returnvalue))
      ;[1 1 1] Get the index number for a new entry and build a string out of it which will be the name of the new save game
      (bind _output_get (LocalVariables|SetSaveGameMetadata _assave_game_metadata_bp)))
    (:Is%20Not%20Valid
      (bind _returnvalue_2 (SaveGame|CreateSaveGameObject "/Game/Blueprints/SaveGameMetadata_BP.SaveGameMetadata_BP_C"))
      (bind _assave_game_metadata_bp_2 (Utilities|Casting|CastToSaveGameMetadata_BP _returnvalue_2))
      (bind _output_get_2 (LocalVariables|SetSaveGameMetadata _assave_game_metadata_bp_2))))
  (bind _nextfreeslot (Default|GetNextFreeSlot _output_get))
  ;[1 1 1] Add a new simple entry to the metadata file
  (Default|AddNewEntry (LocalVariables|GetSaveGameMetadata) (Utilities|String|BuildString(Integer) "SaveGame" "_" _nextfreeslot) (Variables|/Game/Blueprints/SaveGame_BP.SaveGame_BP_C|GetMapName (LocalVariables|GetSaveGameInstance)) (Variables|/Game/Blueprints/SaveGame_BP.SaveGame_BP_C|GetDateTime (LocalVariables|GetSaveGameInstance)))
  ;[1 1 1] Save the metadata file back to memory
  (SaveGame|SaveGametoSlot (LocalVariables|GetSaveGameMetadata) "Metadata")
  (return (Utilities|String|BuildString(Integer) "SaveGame" "_" _nextfreeslot)))

(fn UpdateMetadataEntry
  (params (SaveGame :type Save%20Game%20BP%20Object%20Reference) (SlotName :type String))
  (LocalVariables|SetSaveGameInstance SaveGame)
  (LocalVariables|SetSaveSlotName SlotName)
  (bind _returnvalue (SaveGame|LoadGamefromSlot "metadata"))
  (bind _assave_game_metadata_bp (Utilities|Casting|CastToSaveGameMetadata_BP _returnvalue))
  (bind _output_get (LocalVariables|SetMetadata _assave_game_metadata_bp))
  ;[1 1 1] Loop through the array and search for the entry with the same save game name. When found, set the data and instance name to the new value
  (for (_array_element _array_index) (Variables|/Game/Blueprints/SaveGameMetadata_BP.SaveGameMetadata_BP_C|GetSaveEntries _output_get)
    (if (Utilities|Enum|Equal(Enum) (.SaveGameName (Utilities|Struct|BreakSaveGameSimple _array_element)) (LocalVariables|GetSaveSlotName))
      (Utilities|Array|SetArrayElem (Variables|/Game/Blueprints/SaveGameMetadata_BP.SaveGameMetadata_BP_C|GetSaveEntries (LocalVariables|GetMetadata)) _array_index (Utilities|Struct|MakeSaveGameSimple (LocalVariables|GetSaveSlotName) (Variables|/Game/Blueprints/SaveGame_BP.SaveGame_BP_C|GetMapName (LocalVariables|GetSaveGameInstance)) (Variables|/Game/Blueprints/SaveGame_BP.SaveGame_BP_C|GetDateTime (LocalVariables|GetSaveGameInstance))))
      (SaveGame|SaveGametoSlot (LocalVariables|GetMetadata) "Metadata")
      (return))))

(fn LoadSaveGame
  (bind _asgame_instance_bp (Utilities|Casting|CastToGameInstance_BP (Game|GetGameInstance)))
  (if (not (Variables|/Game/Blueprints/GameInstance_BP.GameInstance_BP_C|GetIsNewGame _asgame_instance_bp))
    (bind _returnvalue (SaveGame|LoadGamefromSlot (Variables|/Game/Blueprints/GameInstance_BP.GameInstance_BP_C|GetSaveGameSlotName _asgame_instance_bp)))
    (bind _assave_game_bp (Utilities|Casting|CastToSaveGame_BP _returnvalue))
    (CallFunction|LoadPlayerStats _assave_game_bp)))

(fn LoadPlayerStats
  (params (SaveGame :type Save%20Game%20BP%20Object%20Reference))
  (LocalVariables|SetSaveGameInstance SaveGame)
  (Transformation|SetActorLocation (Game|Player|GetPlayerPawn 0) (Variables|/Game/Blueprints/SaveGame_BP.SaveGame_BP_C|GetPlayerLocation (LocalVariables|GetSaveGameInstance)) false false)
  (Pawn|SetControlRotation (Game|GetPlayerController 0) (Variables|/Game/Blueprints/SaveGame_BP.SaveGame_BP_C|GetPlayerRotation (LocalVariables|GetSaveGameInstance)))
  (bind _asfirst_person_character_bp (Utilities|Casting|CastToFirstPersonCharacter_BP (Game|Player|GetPlayerPawn 0)))
  (LocalVariables|SetOwningPawn _asfirst_person_character_bp)
  ;[1 1 1] Get loaded ammunition and set the stack size of the equiped weapon to this amount. This will be the ammunition of the gun
  (Variables|/Game/Placeholder_Assets/Actors/ItemBaseClass_Actor.ItemBaseClass_Actor_C|SetStackSize (Variables|/Game/Blueprints/SaveGame_BP.SaveGame_BP_C|GetEquipedWeapon (LocalVariables|GetSaveGameInstance)) (Variables|/Game/Blueprints/SaveGame_BP.SaveGame_BP_C|GetLoadedAmmunition (LocalVariables|GetSaveGameInstance)))
  (Default|EquipWeapon (LocalVariables|GetOwningPawn) (Variables|/Game/Blueprints/SaveGame_BP.SaveGame_BP_C|GetEquipedWeapon (LocalVariables|GetSaveGameInstance)))
  (Variables|/Game/Blueprints/FirstPersonCharacter_BP.FirstPersonCharacter_BP_C|SetInventory (LocalVariables|GetOwningPawn) (Variables|/Game/Blueprints/SaveGame_BP.SaveGame_BP_C|GetPlayerInventory (LocalVariables|GetSaveGameInstance)))
  (Variables|/Game/Blueprints/FirstPersonCharacter_BP.FirstPersonCharacter_BP_C|SetFileStorage (LocalVariables|GetOwningPawn) (Variables|/Game/Blueprints/SaveGame_BP.SaveGame_BP_C|GetPlayerFiles (LocalVariables|GetSaveGameInstance)))
  ;[1 1 1] Load health that was stored for the player and call the changeHealth with 0 health change to set the HUD to the correct value
  (Variables|/Game/Blueprints/FirstPersonCharacter_BP.FirstPersonCharacter_BP_C|SetCurrentHealth (LocalVariables|GetOwningPawn) (Variables|/Game/Blueprints/SaveGame_BP.SaveGame_BP_C|GetCurrentHealth (LocalVariables|GetSaveGameInstance)))
  (Default|ChangeHealth (LocalVariables|GetOwningPawn) 0.0))